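; Test cannonball actor that knocks bricks loose from instanced mesh structures on impact.
; On hit, it removes instances inside a box around the impact and, for BP_BrickImporter targets, adds physics-simulating static meshes in their place, with a delayed self-destroy.
; Overlaps apply radial force to nearby colliding static meshes.
; Tick records location on authority and interpolates remotes toward BallTransform.
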(event `self.ReceiveActorBeginOverlap`
  (params (OtherActor :type "Actor Object Reference"))
  (for _array_element (`self.GetOverlappingComponents` OtherActor)
    (for _array_element_2 (`PrimitiveComponent.GetOverlappingComponents` _array_element)
      (bind _asstatic_mesh_component (cast `StaticMeshComponent` _array_element_2))
      (if (== (`PrimitiveComponent.GetCollisionProfileName` _asstatic_mesh_component) "NoCollision")
        _
        (elif (!= _asstatic_mesh_component (`self.Sphere`))
          (`PrimitiveComponent.AddRadialForce` _asstatic_mesh_component (`SceneComponent.K2_GetComponentLocation` _asstatic_mesh_component) 3000.0 3000000.0 "RIF_Constant" false))))))

(event `self.ReceiveHit`
  (params (MyComp :type "PrimitiveComponent Object Reference") (Other :type "Actor Object Reference") (OtherComp :type "PrimitiveComponent Object Reference") (bSelfMoved :type Boolean) (HitLocation :type "Vector Structure") (HitNormal :type "Vector Structure") (NormalImpulse :type "Vector Structure") (Hit :type "HitResult Structure (by ref)"))
  (bind _hitbox (`self.HitBox`))
  (bind _asinstanced_static_mesh_component (cast `InstancedStaticMeshComponent` OtherComp))
  (bind _returnvalue (`InstancedStaticMeshComponent.GetInstancesOverlappingBox` _asinstanced_static_mesh_component (`KismetMathLibrary.MakeBox` (- HitLocation _hitbox) (+ HitLocation _hitbox)) true))
  (if (!= (`KismetArrayLibrary.Array_Length` _returnvalue) 0)
    (for _array_element _returnvalue
      (bind _output_get (set `self.PartTransformBufer` (`InstancedStaticMeshComponent.GetInstanceTransform` _asinstanced_static_mesh_component _array_element false)))
      (`InstancedStaticMeshComponent.RemoveInstance` _asinstanced_static_mesh_component _array_element)
      (bind _asbp_brick_importer (cast `/Game/Blueprints/NewHyperion/BP_BrickImporter` Other))
      (bind _returnvalue_2 (`AddComponent|NODE_AddStaticMeshComponent-0` :`self` _asbp_brick_importer :`RelativeTransform` _output_get))
      (`StaticMeshComponent.SetStaticMesh` _returnvalue_2 (`StaticMeshComponent.StaticMesh` _asinstanced_static_mesh_component))
      (`PrimitiveComponent.SetCollisionProfileName` _returnvalue_2 "BlockAll" true)
      (`PrimitiveComponent.SetCollisionEnabled` _returnvalue_2 "QueryAndPhysics")
      (`PrimitiveComponent.SetSimulatePhysics` _returnvalue_2 true)
      (`KismetSystemLibrary.Delay` 2.0)
      (`self.K2_DestroyActor`)
      (`PrimitiveComponent.AddRadialForce` _returnvalue_2 HitLocation 30000.0 1000000000.0 "RIF_Constant" true))))

(event `self.ReceiveBeginPlay`
  (`/Engine/EditorBlueprintResources/ActorMacros.Switch Has Authority`))

(event `self.ReceiveTick`
  (params (DeltaSeconds :type "Float (single-precision)"))
  (`/Engine/EditorBlueprintResources/ActorMacros.Switch Has Authority`
    (:`Authority`
      (set `self.BallTransform` (`self.K2_GetActorLocation`)))
    (:`Remote`
      (`self.K2_SetActorLocation` (`KismetMathLibrary.VInterpTo` (`self.K2_GetActorLocation`) (`self.BallTransform`) DeltaSeconds 15.0)))))

(fn `UserConstructionScript`)