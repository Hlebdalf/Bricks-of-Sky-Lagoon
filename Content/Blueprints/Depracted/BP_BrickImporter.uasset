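; Brick importer actor that rebuilds a Lego ship layout from the LegoShipConfig data table in its Construction Script.
; It creates one blocking, frictionless instanced static mesh component per PartsCDA mesh, mapped by the part ID parsed from the mesh name.
; Each table row adds an instance to its part's component, with swapped, negated, MP-scaled coordinates and radian-to-degree rotations.
; Older spawning approaches remain disconnected, and the string Parser function is never called here.
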(event `self.ReceiveBeginPlay`)

(fn `Parser`
  (params (str :type String))
  (returns (Type :type String) (location :type "Vector Structure") (Zrotation :type "Float (double-precision)") (Xrotation :type "Float (double-precision)"))
  (bind _returnvalue (`KismetStringLibrary.ParseIntoArray` str "_"))
  (return (`KismetStringLibrary.Concat_StrStr` (`KismetStringLibrary.Concat_StrStr` "PartsLib_" (`|GetArrayItem` _returnvalue 1)) "PL") (* (`KismetMathLibrary.MakeVector` (`KismetStringLibrary.Conv_StringToDouble` (`KismetStringLibrary.Replace` (`|GetArrayItem` _returnvalue 2) "P" ".")) (`KismetStringLibrary.Conv_StringToDouble` (`KismetStringLibrary.Replace` (`|GetArrayItem` _returnvalue 4) "P" ".")) (`KismetStringLibrary.Conv_StringToDouble` (`KismetStringLibrary.Replace` (`|GetArrayItem` _returnvalue 3) "P" "."))) (`self.MP`)) (`KismetMathLibrary.RadiansToDegrees` (`KismetStringLibrary.Conv_StringToDouble` (`KismetStringLibrary.Replace` (`|GetArrayItem` _returnvalue 6) "P" "."))) (`KismetMathLibrary.RadiansToDegrees` (`KismetStringLibrary.Conv_StringToDouble` (`KismetStringLibrary.Replace` (`|GetArrayItem` _returnvalue 7) "P" ".")))))

(fn `UserConstructionScript`
  (locals (NewLocalVar_0 :type "Float (double-precision)" :default 0.0))
  (for _array_element (`CPDA_PartsData.PartsArray` (`self.PartsCDA`))
    (bind _returnvalue (`AddComponent|NODE_AddInstancedStaticMeshComponent-1`))
    (bind _output (`|GetArrayItem` (`KismetStringLibrary.ParseIntoArray` (`KismetSystemLibrary.GetDisplayName` _array_element) "_") 1))
    (`BlueprintMapLibrary.Map_Add` (`self.PartsDictionary`) (`KismetStringLibrary.GetSubstring` _output 0 (- (`KismetStringLibrary.Len` _output) 2)) _returnvalue)
    (`StaticMeshComponent.SetStaticMesh` _returnvalue _array_element)
    (`PrimitiveComponent.SetCollisionEnabled` _returnvalue "QueryAndPhysics")
    (`PrimitiveComponent.SetCollisionProfileName` _returnvalue "BlockAll" true)
    (`PrimitiveComponent.SetPhysMaterialOverride` _returnvalue "/Game/Materials/noFrictionMaterial.noFrictionMaterial"))
  (bind _outrownames (`DataTableFunctionLibrary.GetDataTableRowNames` "/Game/Datas/LegoShipConfig.LegoShipConfig"))
  (for _array_element_2 _outrownames
    (bind _returnvalue_2 (`|GetDataTableRow` "/Game/Datas/LegoShipConfig.LegoShipConfig" _array_element_2)
      (:`then`
        (bind (_partid _randint _x _y _z _xx _yy _zz) (break `/Game/Datas/PartsShipConfig` _returnvalue_2))
        (bind (_value _returnvalue_3) (`BlueprintMapLibrary.Map_Find` (`self.PartsDictionary`) _partid))
        (if _returnvalue_3
          (`InstancedStaticMeshComponent.AddInstance` _value (`KismetMathLibrary.MakeTransform` (* (`KismetMathLibrary.MakeVector` (* _yy -1.0) (* _xx -1.0) _zz) (`self.MP`)) (`KismetMathLibrary.MakeRotator` (`KismetMathLibrary.RadiansToDegrees` _x) (`KismetMathLibrary.RadiansToDegrees` _z) (`KismetMathLibrary.RadiansToDegrees` _y))) false))))))