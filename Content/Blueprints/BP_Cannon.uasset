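; Cannon actor that launches physics-driven cannonballs when its Fire event is triggered.
; Fire spawns a BP_CannonBall_Test at the Sphere component's transform and applies a mass-dependent impulse along the Arrow's forward vector, scaled by FirePower.
; The IsCanFire flag and a short Delay form a cooldown between shots.
; Nothing in this Blueprint calls Fire, and it has no active BeginPlay, overlap or Tick logic.
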(event `self.Fire`
  (if (`self.isCanFire`)
    (bind _returnvalue (`|SpawnActorFromClass` "/Game/Blueprints/BP_CannonBall_Test.BP_CannonBall_Test_C" (`SceneComponent.K2_GetComponentToWorld` (`self.Sphere`)) "Undefined" "OverrideRootScale" null null))
    (`PrimitiveComponent.AddImpulse` (`/Game/Blueprints/BP_CannonBall_Test.Sphere` _returnvalue) (* (`SceneComponent.GetForwardVector` (`self.Arrow`)) (`self.FirePower`)) "None" false)
    (set `self.isCanFire` false)
    (`KismetSystemLibrary.Delay` 0.5)
    (set `self.isCanFire` true)))

(fn `UserConstructionScript`)