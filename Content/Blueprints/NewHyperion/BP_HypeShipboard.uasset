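; BP_HypeShipboard is a shipboard Blueprint meant to exist as a child actor of a BP_HypeSkyShip.
; On BeginPlay it casts its parent actor to the sky ship and caches it in a SkyShip reference, printing a colored warning if the cast fails.
; It has no other logic of its own: the overlap and tick events are disabled and the construction script only calls its parent.
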(event `self.ReceiveBeginPlay`
  (`parent.ReceiveBeginPlay`)
  (bind _asbp_hype_sky_ship (cast `/Game/Blueprints/NewHyperion/BP_HypeSkyShip` (`self.GetParentActor`))
    (:`then`
      (set `self.SkyShip` _asbp_hype_sky_ship))
    (:`CastFailed`
      (`KismetSystemLibrary.PrintString` "Shipboard doesnt on ship!" true true (struct :`R` 1.0 :`B` 0.244031 :`A` 1.0)))))

(fn `UserConstructionScript`
  (`parent.UserConstructionScript`))