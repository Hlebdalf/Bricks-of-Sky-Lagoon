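; Brick-built ship actor that assembles itself from the LegoShipConfig data table and breaks apart when damaged.
; The construction script creates one instanced mesh component per PartsCDA mesh, maps it by part ID, then adds an instance per table row with converted axes and rotations.
; DamageShip multicasts hit component names; each machine removes instances near the impact.
; Only non-authority machines spawn those bricks as physics debris pushed by a radial impulse.
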(event `DamageShip_Multicast`
  (params (location :type "Vector Structure") (NewParam :type String))
  (bind _returnvalue (* 54.0 3.0))
  (bind _array_element (`self.FindInstance` NewParam))
  (bind _asinstanced_static_mesh_component (cast `InstancedStaticMeshComponent` _array_element))
  (for _array_element_2 (`InstancedStaticMeshComponent.GetInstancesOverlappingSphere` _asinstanced_static_mesh_component location _returnvalue true)
    (bind _output_get (set `self.PartTransformBufer` (`InstancedStaticMeshComponent.GetInstanceTransform` _asinstanced_static_mesh_component _array_element_2 false)))
    (`InstancedStaticMeshComponent.RemoveInstance` _asinstanced_static_mesh_component _array_element_2)
    (`/Engine/EditorBlueprintResources/ActorMacros.Switch Has Authority`
      (:`Remote`
        (bind _returnvalue_2 (`AddComponent|NODE_AddStaticMeshComponent-7` :`RelativeTransform` _output_get))
        (`StaticMeshComponent.SetStaticMesh` _returnvalue_2 (`StaticMeshComponent.StaticMesh` _asinstanced_static_mesh_component))
        (`PrimitiveComponent.SetCollisionProfileName` _returnvalue_2 "NoCollision" true)
        (`PrimitiveComponent.SetCollisionEnabled` _returnvalue_2 "PhysicsOnly")
        (`PrimitiveComponent.SetSimulatePhysics` _returnvalue_2 true)
        (`PrimitiveComponent.AddRadialImpulse` _returnvalue_2 location (* _returnvalue 5.0) 500000.0 "RIF_Constant" false)))))

(event `self.DamageShip`
  (params (location :type "Vector Structure") (CollectedComponents :type "Array of PrimitiveComponent Object Reference (by ref)"))
  (bind _instancename (`self.InstanceName`))
  (`KismetArrayLibrary.Array_Clear` (`self.InstanceName`))
  (for _array_element CollectedComponents
    (cast `InstancedStaticMeshComponent` _array_element)
    (bind _returnvalue (`KismetArrayLibrary.Array_AddUnique` _instancename (`KismetSystemLibrary.GetDisplayName` _array_element)))
    (`self.DamageShip_Multicast` location (`|GetArrayItem` _instancename _returnvalue))))

(event `self.ReceiveBeginPlay`
  (`/Engine/EditorBlueprintResources/ActorMacros.Switch Has Authority`
    (:`Authority`
      (for _array_element _
        (`SceneComponent.SetVisibility` _array_element false false)))))

(fn `FindInstance`
  (params (B :type String))
  (returns (`Array Element` :type "SceneComponent Object Reference"))
  (for _array_element (`SceneComponent.GetChildrenComponents` (`self.Arrow`) false)
    (if (== (`KismetSystemLibrary.GetDisplayName` _array_element) B)
      (return _array_element))))

(fn `OnRep_Somehing`)

(fn `Parser`
  (params (str :type String))
  (returns (Type :type String) (location :type "Vector Structure") (Zrotation :type "Float (double-precision)") (Xrotation :type "Float (double-precision)"))
  (bind _returnvalue (`KismetStringLibrary.ParseIntoArray` str "_"))
  (return (`KismetStringLibrary.Concat_StrStr` (`KismetStringLibrary.Concat_StrStr` "PartsLib_" (`|GetArrayItem` _returnvalue 1)) "PL") (* (`KismetMathLibrary.MakeVector` (`KismetStringLibrary.Conv_StringToDouble` (`KismetStringLibrary.Replace` (`|GetArrayItem` _returnvalue 2) "P" ".")) (`KismetStringLibrary.Conv_StringToDouble` (`KismetStringLibrary.Replace` (`|GetArrayItem` _returnvalue 4) "P" ".")) (`KismetStringLibrary.Conv_StringToDouble` (`KismetStringLibrary.Replace` (`|GetArrayItem` _returnvalue 3) "P" "."))) (`self.MP`)) (`KismetMathLibrary.RadiansToDegrees` (`KismetStringLibrary.Conv_StringToDouble` (`KismetStringLibrary.Replace` (`|GetArrayItem` _returnvalue 6) "P" "."))) (`KismetMathLibrary.RadiansToDegrees` (`KismetStringLibrary.Conv_StringToDouble` (`KismetStringLibrary.Replace` (`|GetArrayItem` _returnvalue 7) "P" ".")))))

(fn `UserConstructionScript`
  (locals (NewLocalVar_0 :type "Float (double-precision)" :default 0.0))
  (for _array_element (`CPDA_PartsData.PartsArray` (`self.PartsCDA`))
    (bind _returnvalue (`AddComponent|NODE_AddInstancedStaticMeshComponent-1`))
    (bind _output (`|GetArrayItem` (`KismetStringLibrary.ParseIntoArray` (`KismetSystemLibrary.GetDisplayName` _array_element) "_") 1))
    (`BlueprintMapLibrary.Map_Add` (`self.PartsDictionary`) (`KismetStringLibrary.GetSubstring` _output 0 (- (`KismetStringLibrary.Len` _output) 2)) _returnvalue)
    (`StaticMeshComponent.SetStaticMesh` _returnvalue _array_element)
    (`PrimitiveComponent.SetCollisionEnabled` _returnvalue "QueryAndPhysics")
    (`PrimitiveComponent.SetCollisionProfileName` _returnvalue "BlockAll" true)
    (`PrimitiveComponent.SetPhysMaterialOverride` _returnvalue null))
  (bind _outrownames (`DataTableFunctionLibrary.GetDataTableRowNames` "/Game/Datas/LegoShipConfig.LegoShipConfig"))
  (for _array_element_2 _outrownames
    (bind _returnvalue_2 (`|GetDataTableRow` "/Game/Datas/LegoShipConfig.LegoShipConfig" _array_element_2)
      (:`then`
        (bind (_partid _randint _x _y _z _xx _yy _zz) (break `/Game/Datas/PartsShipConfig` _returnvalue_2))
        (bind (_value _returnvalue_3) (`BlueprintMapLibrary.Map_Find` (`self.PartsDictionary`) _partid))
        (if _returnvalue_3
          (`InstancedStaticMeshComponent.AddInstance` _value (`KismetMathLibrary.MakeTransform` (* (`KismetMathLibrary.MakeVector` (* _yy -1.0) (* _xx -1.0) _zz) (`self.MP`)) (`KismetMathLibrary.MakeRotator` (`KismetMathLibrary.RadiansToDegrees` _x) (`KismetMathLibrary.RadiansToDegrees` _z) (`KismetMathLibrary.RadiansToDegrees` _y))) false))))))