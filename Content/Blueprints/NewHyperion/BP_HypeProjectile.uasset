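; BP_HypeProjectile is a projectile that breaks apart instanced-mesh brick structures where it hits.
; On hit, it finds instances in a sphere scaled from its capsule radius, saves their transforms and removes them.
; When the hit actor is a BP_BrickImporter, each removed instance becomes a physics-simulating StaticMeshComponent on that actor, pushed by a radial impulse.
; The projectile destroys itself shortly after hitting an instanced mesh.
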(event `self.ReceiveActorBeginOverlap`
  (params (OtherActor :type "Actor Object Reference")))

(event `self.ReceiveHit`
  (params (MyComp :type "PrimitiveComponent Object Reference") (Other :type "Actor Object Reference") (OtherComp :type "PrimitiveComponent Object Reference") (bSelfMoved :type Boolean) (HitLocation :type "Vector Structure") (HitNormal :type "Vector Structure") (NormalImpulse :type "Vector Structure") (Hit :type "HitResult Structure (by ref)"))
  (bind _asinstanced_static_mesh_component (cast `InstancedStaticMeshComponent` OtherComp))
  (for _array_element (`InstancedStaticMeshComponent.GetInstancesOverlappingSphere` _asinstanced_static_mesh_component HitLocation (* (`CapsuleComponent.GetScaledCapsuleRadius` (`self.Capsule`)) 2.0) true)
    (bind _output_get (set `self.PartTransformBufer` (`InstancedStaticMeshComponent.GetInstanceTransform` _asinstanced_static_mesh_component _array_element false)))
    (`InstancedStaticMeshComponent.RemoveInstance` _asinstanced_static_mesh_component _array_element)
    (`/Engine/EditorBlueprintResources/ActorMacros.Switch Has Authority`
      (:`Authority`
        _)
      (:`Remote`
        _))
    (bind _asbp_brick_importer (cast `/Game/Blueprints/NewHyperion/BP_BrickImporter` Other))
    (bind _returnvalue (`AddComponent|NODE_AddStaticMeshComponent-0` :`self` _asbp_brick_importer :`RelativeTransform` _output_get))
    (`StaticMeshComponent.SetStaticMesh` _returnvalue (`StaticMeshComponent.StaticMesh` _asinstanced_static_mesh_component))
    (`PrimitiveComponent.SetSimulatePhysics` _returnvalue true)
    (`PrimitiveComponent.AddRadialImpulse` _returnvalue HitLocation 600.0 400000.0 "RIF_Constant" false))
  (`KismetSystemLibrary.Delay` 0.1)
  (`self.K2_DestroyActor`))

(fn `UserConstructionScript`)