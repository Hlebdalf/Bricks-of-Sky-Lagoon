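; BP_HypeCanon is a networked cannon that aims its mesh and launches projectiles along its Arrow at Firepower.
; DoSomething calls Fire when IsCanFire is set; the authority spawns a HypeProjectile and runs the ReloadTime cooldown.
; Remote instances spawn a BP_FakeProjectile with the same impulse and no cooldown of their own.
; Tick drives mesh yaw and roll from Value, directly on authority and smoothed with FInterpTo on remotes.
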(event `SpawnProjectiles`
  (bind _arrow (`self.Arrow`))
  (bind _arrow_2 (`self.Arrow`))
  (`/Engine/EditorBlueprintResources/ActorMacros.Switch Has Authority`
    (:`Authority`
      (bind _returnvalue (`|SpawnActorFromClass` "/Script/Hyperion.HypeProjectile" (`SceneComponent.K2_GetComponentToWorld` _arrow) "Undefined" "OverrideRootScale" null null))
      (`HypeProjectile.AddProjectileImpulse` _returnvalue (* (`SceneComponent.GetForwardVector` _arrow) (`self.Firepower`)))
      (set `self.bIsCanFire` false)
      (`KismetSystemLibrary.Delay` (`self.ReloadTime`))
      (set `self.bIsCanFire` true))
    (:`Remote`
      (bind _returnvalue_2 (`|SpawnActorFromClass` "/Game/Blueprints/NewHyperion/BP_FakeProjectile.BP_FakeProjectile_C" (`SceneComponent.K2_GetComponentToWorld` _arrow_2) "Undefined" "OverrideRootScale" null null))
      (`PrimitiveComponent.AddImpulse` (`/Game/Blueprints/NewHyperion/BP_FakeProjectile.Capsule` _returnvalue_2) (* (`SceneComponent.GetForwardVector` _arrow_2) (`self.Firepower`)) "None" false))))

(event `Fire`
  (`self.SpawnProjectiles`))

(event `/Game/Blueprints/NewHyperion/BP_HypeInteractive.DoSomething`
  (if (`self.bIsCanFire`)
    (`self.Fire`)))

(event `self.ReceiveTick`
  (params (DeltaSeconds :type "Float (single-precision)"))
  (bind _returnvalue (`GameplayStatics.GetWorldDeltaSeconds`))
  (bind (_value_x _value_y) (`KismetMathLibrary.BreakVector2D` (`self.Value`)))
  (bind _staticmesh (`self.StaticMesh`))
  (bind (_value_x_2 _value_y_2) (`KismetMathLibrary.BreakVector2D` (`self.Value`)))
  (bind (_relativerotation_roll _relativerotation_pitch _relativerotation_yaw) (`KismetMathLibrary.BreakRotator` (`SceneComponent.RelativeRotation` (`self.StaticMesh`))))
  (`parent.ReceiveTick` DeltaSeconds)
  (`/Engine/EditorBlueprintResources/ActorMacros.Switch Has Authority`
    (:`Authority`
      (`SceneComponent.K2_SetRelativeRotation` _staticmesh (`KismetMathLibrary.MakeRotator` _value_y 0.0 _value_x) false false))
    (:`Remote`
      (`SceneComponent.K2_SetRelativeRotation` _staticmesh (`KismetMathLibrary.MakeRotator` (`KismetMathLibrary.FInterpTo` _relativerotation_roll _value_y_2 _returnvalue 15.0) 0.0 (`KismetMathLibrary.FInterpTo` _relativerotation_yaw _value_x_2 _returnvalue 15.0)) false false))))

(fn `UserConstructionScript`
  (`parent.UserConstructionScript`))