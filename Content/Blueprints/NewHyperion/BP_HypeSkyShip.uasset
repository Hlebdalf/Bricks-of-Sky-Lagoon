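; BP_HypeSkyShip is a physics-driven sky ship that hovers around an adjustable target height.
; On authority, four buoy points push the Cube body in proportion to their height error, and a settable torque yaws it.
; Authority records ShipTransform each tick, while remotes disable physics and interpolate toward it.
; It also tracks its previous and current location to expose a per-tick movement delta.
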(event `self.ReceiveBeginPlay`
  (`/Engine/EditorBlueprintResources/ActorMacros.Switch Has Authority`
    (:`Authority`
      (set `self.TargetFloor` (`self.Floor`))
      (bind _output_get (set `self.PreLocation` (`self.K2_GetActorLocation`)))
      (set `self.NowLocation` _output_get))
    (:`Remote`
      (`PrimitiveComponent.SetSimulatePhysics` (`self.Cube`) false))))

(event `self.ReceiveTick`
  (params (DeltaSeconds :type "Float (single-precision)"))
  (`/Engine/EditorBlueprintResources/ActorMacros.Switch Has Authority`
    (:`Authority`
      (`|ExecutionSequence`
        (:`then_0`
          (for _array_element (`|MakeArray` (`self.Bouy2`) (`self.Bouy3`) (`self.Bouy4`) (`self.Bouy1`))
            (bind (_returnvalue_x _returnvalue_y _returnvalue_z) (`KismetMathLibrary.BreakVector` (`SceneComponent.K2_GetComponentLocation` _array_element)))
            (`PrimitiveComponent.AddForceAtLocationLocal` (`self.Cube`) (`KismetMathLibrary.MakeVector` 0.0 0.0 (* (- (`self.TargetFloor`) _returnvalue_z) (`self.ArchimedesForceMP`))) (`SceneComponent.RelativeLocation` _array_element) "None")))
        (:`then_1`
          (set `self.PreLocation` (`self.NowLocation`))
          (set `self.NowLocation` (`self.K2_GetActorLocation`)))
        (:`then_2`
          (`PrimitiveComponent.AddTorqueInRadians` (`self.Cube`) (`KismetMathLibrary.MakeVector` 0.0 0.0 (`self.Torque`)) "None" false))
        (:`then_3`
          (set `self.ShipTransform` (`self.GetTransform`)))))
    (:`Remote`
      (`self.K2_SetActorTransform` (`KismetMathLibrary.TInterpTo` (`self.GetTransform`) (`self.ShipTransform`) DeltaSeconds 5.0)))))

(event `SetTargetFloor`
  (params (value :type "Float (double-precision)"))
  (set `self.TargetFloor` (+ (`self.Floor`) value)))

(event `SetTorque`
  (params (value :type "Float (double-precision)"))
  (bind _output_get (set `self.Torque` value)))

(fn `GetDeltaLocation`
  (returns (NewParam :type "Vector Structure"))
  (return (- (`self.NowLocation`) (`self.PreLocation`))))

(fn `UserConstructionScript`)