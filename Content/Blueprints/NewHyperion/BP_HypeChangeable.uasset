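; BP_HypeChangeable is an actor Blueprint that holds a two-axis Value, adjusted by axis input through its SetX and SetY events.
; Each event runs on authority only, scales the input by AxisMP and adds it to the current component.
; Results strictly between Floor and Roof are stored in XInput or YInput, and a shared step rebuilds Value from both; out-of-range changes are ignored rather than clamped.
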(event `SetX`
  (params (axis :type "Float (double-precision)"))
  (bind (_axismp_x _axismp_y) (`KismetMathLibrary.BreakVector2D` (`self.AxisMP`)))
  (bind (_value_x _value_y) (`KismetMathLibrary.BreakVector2D` (`self.Value`)))
  (bind (_floor_x _floor_y) (`KismetMathLibrary.BreakVector2D` (`self.Floor`)))
  (bind (_roof_x _roof_y) (`KismetMathLibrary.BreakVector2D` (`self.Roof`)))
  (bind _returnvalue (+ (* axis _axismp_x) _value_x))
  (`/Engine/EditorBlueprintResources/ActorMacros.Switch Has Authority`
    (:`Authority`
      (if (and (< _returnvalue _roof_x) (> _returnvalue _floor_x))
        (bind _output_get (set `self.XInput` _returnvalue))
        (set `self.Value` (`KismetMathLibrary.MakeVector2D` _output_get (stale `SetY` _output_get)) :!label _label)))))

(event `SetY`
  (params (axis :type "Float (double-precision)"))
  (bind (_axismp_x _axismp_y) (`KismetMathLibrary.BreakVector2D` (`self.AxisMP`)))
  (bind (_value_x _value_y) (`KismetMathLibrary.BreakVector2D` (`self.Value`)))
  (bind (_floor_x _floor_y) (`KismetMathLibrary.BreakVector2D` (`self.Floor`)))
  (bind (_roof_x _roof_y) (`KismetMathLibrary.BreakVector2D` (`self.Roof`)))
  (bind _returnvalue (+ _value_y (* _axismp_y axis)))
  (`/Engine/EditorBlueprintResources/ActorMacros.Switch Has Authority`
    (:`Authority`
      (if (and (< _returnvalue _roof_y) (> _returnvalue _floor_y))
        (bind _output_get (set `self.YInput` _returnvalue))
        (goto _label)))))

(fn `UserConstructionScript`
  (`parent.UserConstructionScript`))